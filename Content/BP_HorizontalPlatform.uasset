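; BP_HorizontalPlatform is a platform actor set up to move toward a target actor, though this file only precomputes the movement values.
; The construction script converts Speed from km/h to cm/s, stores the distance to TargetActor as MaxDistance, and scales the normalized direction to it into PlatformVelocity.
; Distance and velocity helpers compute only when TargetActor is valid, and the event graph contains no movement logic.
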(event `self.ReceiveBeginPlay`)

(fn `ConvertToCentimeterPerSecond`
  (returns (ReturnValue :type "Float (double-precision)"))
  (return (* (/ (`self.Speed`) 3.6) 100.0)))

(fn `GetCalculatedVelocity`
  (returns (ReturnValue :type "Vector Structure"))
  (bind _targetactor (`self.TargetActor`)
    (:`then`
      (return (* (`KismetMathLibrary.Normal` (- (`self.K2_GetActorLocation` _targetactor) (`self.K2_GetActorLocation`))) (`self.Speed In cm/s`))))
    (:`else`)))

(fn `GetMaxDistance`
  (returns (ReturnValue :type "Float (double-precision)"))
  (bind _targetactor (`self.TargetActor`)
    (:`then`
      (return (`KismetMathLibrary.Vector_Distance` (`self.K2_GetActorLocation` _targetactor) (`self.K2_GetActorLocation`))))
    (:`else`)))

(fn `UserConstructionScript`
  (set `self.Speed In cm/s` (`self.ConvertToCentimeterPerSecond`))
  (set `self.MaxDistance` (`self.GetMaxDistance`))
  (set `self.PlatformVelocity` (`self.GetCalculatedVelocity`)))